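; Sonar blip actor that animates its decal, apparently as a sonar pulse effect, when triggered by contact.
; An overlap from the FirstPersonCharacter, or a hit on its box component, restarts a timeline from the beginning.
; The timeline lerps the decal's relative transform between two stored transforms.
; A second timeline that moves only the decal's location is left unconnected and never runs.
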(event `self.ReceiveActorBeginOverlap`
  (params (OtherActor :type "Actor Object Reference"))
  (cast `/Game/FirstPersonBP/Blueprints/FirstPersonCharacter` OtherActor)
  (bind (_direction _newtrack_0) (`Timeline|Timeline_0` :!via `PlayFromStart` :!label _label)
    (:`Update`
      (`SceneComponent.K2_SetRelativeTransform` (`self.Decal`) (`KismetMathLibrary.TLerp` (`self.NewVar_0`) (`self.NewVar_1`) _newtrack_0) false false))))

(event `self.Box.OnComponentHit`
  (params (HitComponent :type "PrimitiveComponent Object Reference") (OtherActor :type "Actor Object Reference") (OtherComp :type "PrimitiveComponent Object Reference") (NormalImpulse :type "Vector Structure") (Hit :type "HitResult Structure (by ref)"))
  (cast `BoxComponent` HitComponent)
  (goto _label :!via `PlayFromStart`))

(fn `UserConstructionScript`)